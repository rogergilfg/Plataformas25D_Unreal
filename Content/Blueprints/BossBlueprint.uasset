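; Boss enemy that spots the GordoBorracho player via PawnSensing, chases with AI MoveTo every Tick and plays an attack montage on arrival.
; Right-hand collision, toggled by custom events, deals damage on overlap.
; Hits play montage and sound; first dropping to low, nonzero life sets ModeBoss and refills health, leaving OnHit set, which blocks attacks.
; ActivarEscoba, uncalled here, draws the broom and enables its collision.
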(event OnSeePawn(PawnSensing)
  (params (Pawn :type Pawn%20Object%20Reference))
  ;[0.15 0.15 0.15 0.5] Follow
  (if (not (Variables|Default|GetDeath))
    (if (not (Variables|Default|GetIsPunching))
      (bind _asgordo_borracho (Utilities|Casting|CastToGordoBorracho Pawn))
      (Variables|Default|SetPlayerDetected true))))

(event OnComponentBeginOverlap(Right)
  (params (OverlappedComponent :type Primitive%20Component%20Object%20Reference) (OtherActor :type Actor%20Object%20Reference) (OtherComp :type Primitive%20Component%20Object%20Reference) (OtherBodyIndex :type Integer) (bFromSweep :type Boolean) (SweepResult :type Hit%20Result%20Structure%20%28by%20ref%29))
  ;[0.15 0.15 0.15 0.5] CollisionsCombat
  (bind _asgordo_borracho (Utilities|Casting|CastToGordoBorracho OtherActor))
  (Default|TakeDamage _asgordo_borracho (Variables|Default|GetDamage)))

(event Custom|FOLLOW
  (params (Player :type Character%20Object%20Reference))
  ;[0.15 0.15 0.15 0.5] Follow
  (AI|AIMoveTo self "0, 0, 0" Player 1.1e+02 false
    (:OnSuccess
      (CallFunction|Combate))))

(event Custom|ActivarRight
  ;[0.15 0.15 0.15 0.5] CollisionsCombat
  (Collision|SetCollisionEnabled (Variables|Default|GetRight) "QueryOnly"))

(event Custom|TakeDamage
  (params (Damage :type Float%20%28double-precision%29))
  ;[0.15 0.15 0.15 0.5] TakeDamage
  (Variables|Default|SetOnHit true)
  (bind _output_get (Variables|Default|SetLife (- (Variables|Default|GetLife) Damage)))
  (if (<= _output_get 0.0)
    (Variables|Default|SetDeath true)
    (else
      (Utilities|Casting|CastToGordoBorracho (Game|GetPlayerCharacter 0))
      (Animation|PlayAnimMontage "/Game/Boss/Animaciones/Hit.Hit" 1.0 "None")
      (Audio|PlaySoundatLocation "/Game/SFX/punch-notification_sound-493565.punch-notification_sound-493565" "0, 0, 0" "0, 0, 0" 0.75 1.0 0.08 0 0 0 0)
      (Development|PrintString "GOLPE")
      (if (<= (Variables|Default|GetLife) 3e+01)
        (if (Variables|Default|GetModeBoss)
          (Variables|Default|SetOnHit false)
          (else
            (Variables|Default|SetModeBoss true)
            (Variables|Default|SetLife 1e+02)))
        (else
          (Variables|Default|SetOnHit false))))))

(event Custom|Combate
  ;[0.15 0.15 0.15 0.5] Combat
  (if (not (Variables|Default|GetOnHit))
    (Variables|Default|SetIsPunching true)
    (bind _returnvalue (Animation|PlayAnimMontage "/Game/Boss/Animaciones/Attack.Attack" 1.0 "None"))
    (Utilities|FlowControl|Delay _returnvalue)
    (Variables|Default|SetIsPunching false)))

(event Custom|DesactivarRight
  ;[0.15 0.15 0.15 0.5] CollisionsCombat
  (Collision|SetCollisionEnabled (Variables|Default|GetRight) "NoCollision"))

(event Custom|DesactivarEscoba
  ;[0.15 0.15 0.15 0.5] CollisionsCombat
  (Collision|SetCollisionEnabled (Variables|Default|GetSphere1) "NoCollision"))

(event Custom|ActivarEscoba
  ;[0.15 0.15 0.15 0.5] CollisionsCombat
  (Rendering|SetVisibility (Variables|Default|GetEscobaCintura) false false)
  (Rendering|SetVisibility (Variables|Default|GetEscobaBoss) true false)
  (Collision|SetCollisionEnabled (Variables|Default|GetSphere1) "QueryOnly")
  (Animation|PlayAnimMontage "/Game/Boss/Animaciones/Desenfundar.Desenfundar" 1.0 "None"))

(event EventBeginPlay
  (CallFunction|DesactivarRight)
  (CallFunction|DesactivarEscoba))

(event Collision|EventActorBeginOverlap
  (params (OtherActor :type Actor%20Object%20Reference)))

(event EventTick
  (params (DeltaSeconds :type Float%20%28single-precision%29))
  ;[0.15 0.15 0.15 0.5] Follow
  (if (Variables|Default|GetPlayerDetected)
    (if (not (Variables|Default|GetIsPunching))
      (if (not (Variables|Default|GetDeath))
        (if (not (Variables|/Game/Blueprints/GordoBorracho.GordoBorracho_C|GetMuerte (stale OnSeePawn(PawnSensing) _asgordo_borracho)))
          (CallFunction|FOLLOW (stale OnSeePawn(PawnSensing) _asgordo_borracho)))))))

(fn ConstructionScript)

(fn COMBAT)