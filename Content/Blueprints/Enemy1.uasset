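; Melee enemy that chases and punches the GordoBorracho player character.
; PawnSensing sets the target, then Tick repeatedly issues AIMoveTo until in range, where an attack montage plays.
; Hand colliders, switched by activate/deactivate events, apply damage on overlap.
; Incoming damage reduces life, setting Muerte (dead) at zero to halt behavior, otherwise playing a head or lateral hit reaction based on player combo and hit side.
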(event OnSeePawn(PawnSensing)
  (params (Pawn :type Pawn%20Object%20Reference))
  ;[0.15 0.15 0.15 0.5] Follow
  (if (not (Variables|Default|GetMuerte))
    (if (not (Variables|Default|GetIsPunching))
      (bind _asgordo_borracho (Utilities|Casting|CastToGordoBorracho Pawn))
      (Variables|Default|SetPlayerDetected true))))

(event OnComponentBeginOverlap(LeftHand)
  (params (OverlappedComponent :type Primitive%20Component%20Object%20Reference) (OtherActor :type Actor%20Object%20Reference) (OtherComp :type Primitive%20Component%20Object%20Reference) (OtherBodyIndex :type Integer) (bFromSweep :type Boolean) (SweepResult :type Hit%20Result%20Structure%20%28by%20ref%29))
  ;[0.15 0.15 0.15 0.5] CombatColliders
  (bind _asgordo_borracho (Utilities|Casting|CastToGordoBorracho OtherActor))
  (Default|TakeDamage _asgordo_borracho (Variables|Default|GetDamage)))

(event OnComponentBeginOverlap(RightHand)
  (params (OverlappedComponent :type Primitive%20Component%20Object%20Reference) (OtherActor :type Actor%20Object%20Reference) (OtherComp :type Primitive%20Component%20Object%20Reference) (OtherBodyIndex :type Integer) (bFromSweep :type Boolean) (SweepResult :type Hit%20Result%20Structure%20%28by%20ref%29))
  ;[0.15 0.15 0.15 0.5] CombatColliders
  (bind _asgordo_borracho (Utilities|Casting|CastToGordoBorracho OtherActor))
  (Default|TakeDamage _asgordo_borracho (Variables|Default|GetDamage)))

(event Custom|FOLLOW
  (params (Player :type Character%20Object%20Reference))
  ;[0.15 0.15 0.15 0.5] Follow
  (AI|AIMoveTo self "0, 0, 0" Player 1.1e+02 false
    (:OnSuccess
      (CallFunction|COMBAT))))

(event Custom|COMBAT
  ;[0.15 0.15 0.15 0.5] Combat
  (if (not (Variables|Default|GetOnHit))
    (if (not (Variables|Default|GetMuerte))
      (Variables|Default|SetIsPunching true)
      (bind _returnvalue (Animation|PlayAnimMontage "/Game/Enemy/Animaciones/Attack.Attack" 1.0 "None"))
      (Utilities|FlowControl|Delay _returnvalue)
      (Variables|Default|SetIsPunching false))))

(event Custom|DesactivatePunchColliderLeft
  ;[0.15 0.15 0.15 0.5] CombatColliders
  (Collision|SetCollisionEnabled (Variables|Default|GetLeftHand) "NoCollision"))

(event Custom|TakeDamage
  (params (Damage :type Float%20%28double-precision%29) (Right :type Boolean))
  ;[0.15 0.15 0.15 0.5] TakeDamage
  (Variables|Default|SetOnHit true)
  (bind _output_get (Variables|Default|SetLife (- (Variables|Default|GetLife) Damage)))
  (if (<= _output_get 0.0)
    (Variables|Default|SetMuerte true)
    (else
      (bind _asgordo_borracho (Utilities|Casting|CastToGordoBorracho (Game|GetPlayerCharacter 0)))
      (if (>= (Variables|/Game/Blueprints/GordoBorracho.GordoBorracho_C|GetCombo _asgordo_borracho) 3)
        (if Right
          (Animation|PlayAnimMontage "/Game/Enemy/Animaciones/LateralHit.LateralHit" 1.0 "None")
          (Audio|PlaySoundatLocation "/Game/SFX/strongpunch_1.strongpunch_1" "0, 0, 0" "0, 0, 0" 0.75 1.0 0.08 0 0 0 0)
          (Variables|Default|SetOnHit false)
          (else
            (Animation|PlayAnimMontage "/Game/Enemy/Animaciones/Head_Hit_Montage.Head_Hit_Montage" 1.0 "None" :!label _label)
            (Audio|PlaySoundatLocation "/Game/SFX/punch-notification_sound-493565.punch-notification_sound-493565" "0, 0, 0" "0, 0, 0" 1.0 1.0 0.08 0 0 0 0)
            (Variables|Default|SetOnHit false)))
        (else
          (goto _label))))))

(event Custom|DesactivatePunchColliderRight
  ;[0.15 0.15 0.15 0.5] CombatColliders
  (Collision|SetCollisionEnabled (Variables|Default|GetRightHand) "NoCollision"))

(event Custom|ActivatePunchColliderRight
  ;[0.15 0.15 0.15 0.5] CombatColliders
  (Collision|SetCollisionEnabled (Variables|Default|GetRightHand) "QueryOnly"))

(event Custom|ActivatePunchColliderLeft
  ;[0.15 0.15 0.15 0.5] CombatColliders
  (Collision|SetCollisionEnabled (Variables|Default|GetLeftHand) "QueryOnly"))

(event EventBeginPlay
  (CallFunction|DesactivatePunchColliderRight)
  (CallFunction|DesactivatePunchColliderLeft))

(event Collision|EventActorBeginOverlap
  (params (OtherActor :type Actor%20Object%20Reference)))

(event EventTick
  (params (DeltaSeconds :type Float%20%28single-precision%29))
  ;[0.15 0.15 0.15 0.5] Follow
  (if (Variables|Default|GetPlayerDetected)
    (if (not (Variables|Default|GetIsPunching))
      (if (not (Variables|Default|GetMuerte))
        (if (not (Variables|/Game/Blueprints/GordoBorracho.GordoBorracho_C|GetMuerte (stale OnSeePawn(PawnSensing) _asgordo_borracho)))
          (CallFunction|FOLLOW (stale OnSeePawn(PawnSensing) _asgordo_borracho)))))))

(fn ConstructionScript)